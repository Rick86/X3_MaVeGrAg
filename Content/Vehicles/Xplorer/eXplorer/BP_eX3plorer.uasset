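; BP_eX3plorer is a child vehicle Blueprint, an eXplorer variant in the Xplorer family that relies on its parent class for behavior.
; Its lifecycle, overlap, significance, multicast trunk open and close events, and construction script only call the parent versions.
; The remaining custom events, with inputs such as delta time, key, axis value and flashlight state, are empty, so the graphs add no logic of their own.
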(event Custom|CustomEvent
  (params (InDeltaTime :type Float%20%28single-precision%29)))

(event Custom|CustomEvent_1)

(event Custom|CustomEvent_2
  (params (Key :type Key%20Structure :default "None")))

(event Custom|CustomEvent_3
  (params (AxisValue :type Float%20%28single-precision%29)))

(event Custom|CustomEvent_4
  (params (FlashlightOn :type Boolean)))

(event EventBeginPlay
  (|CallParentFunction))

(event Collision|EventActorBeginOverlap
  (params (OtherActor :type Actor%20Object%20Reference))
  (|CallParentFunction OtherActor))

(event EventTick
  (params (DeltaSeconds :type Float%20%28single-precision%29))
  (|CallParentFunction DeltaSeconds))

(event EventGainedSignificance
  (|CallParentFunction))

(event EventLostSignificance
  (|CallParentFunction))

(event EventMulticastOpenTrunk
  (|CallParentFunction))

(event EventMulticastCloseTrunk
  (|CallParentFunction))

(fn ConstructionScript
  (|CallParentFunction))