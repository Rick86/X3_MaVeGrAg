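; Mk1 X3 drone station that draws extra power to recharge a drone each time it docks, scaled to the length of its trip.
; StartDockingSequence runs the parent logic, then takes the latest round-trip time, falling back to the estimate, or only logs if neither exceeds PowerConsumptionIdle.
; It spreads the trip's battery energy over a fixed charging window, raising target consumption after a docking delay and restoring idle afterward.
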(event EventStartDockingSequence
  (params (Drone :type FG%20Drone%20Vehicle%20Object%20Reference))
  (|CallParentFunction Drone)
  ;[1 1 1] Get Trip Time
  (Variables|Default|SetTripTime 0.0) ; Reset trip time
  (if (> (Class|FGDroneStationInfo|GetLatestRoundTripTime (Class|FGBuildableDroneStation|GetInfo self)) (Variables|Default|GetPowerConsumptionIdle)) ; If we have Latest round trip
    (bind _output_get (Variables|Default|SetTripTime (Class|FGDroneStationInfo|GetLatestRoundTripTime (Class|FGBuildableDroneStation|GetInfo))))
    (CallFunction|DEBUG (Utilities|String|Append "Trip Time (last round): " (Utilities|String|ToString(Float) _output_get)) true "(R=0.000000,G=0.031200,B=0.375000,A=1.000000)")
    ;[1 1 1] Calculate Recharge Power-Consumption
    (Variables|Default|SetPowerConsumptionForCharging (/ (* (Variables|Default|GetPowerConsumptionBatteryMwh) (Variables|Default|GetTripTime)) 2e+01) :!label _label)
    (CallFunction|DEBUG (Utilities|String|Append "Recharge Power-Consumptio will be " (Utilities|String|ToString(Float) (/ (* (Variables|Default|GetPowerConsumptionBatteryMwh) (Variables|Default|GetTripTime)) 2e+01))) true "(R=0.000000,G=0.031200,B=0.375000,A=1.000000)")
    (Utilities|FlowControl|Delay 14.0) ; Wait until it really docked
    ;[1 1 1] Start Recharge Process
    (CallFunction|DEBUG (Utilities|String|Append "START Recharge, set consumption to " (Utilities|String|ToString(Float) (Variables|Default|GetPowerConsumptionForCharging)) " (20 seconds from now)") true "(R=0.000000,G=0.031200,B=0.375000,A=1.000000)")
    (Class|FGPowerInfoComponent|SetTargetConsumption (Class|FGBuildableFactory|GetPowerInfo self) (Variables|Default|GetPowerConsumptionForCharging))
    (Utilities|FlowControl|Delay 2e+01) ; Wait 20 seconds, until the\nfull docking process is done
    (CallFunction|DEBUG (Utilities|String|Append "END Recharge, set consumption back to " (Utilities|String|ToString(Float) (Variables|Default|GetPowerConsumptionIdle))) true "(R=0.000000,G=0.031200,B=0.375000,A=1.000000)")
    (Class|FGPowerInfoComponent|SetTargetConsumption (Class|FGBuildableFactory|GetPowerInfo self) (Variables|Default|GetPowerConsumptionIdle))
    (elif (> (Class|FGDroneStationInfo|GetEstimatedRoundTripTime (Class|FGBuildableDroneStation|GetInfo self)) (Variables|Default|GetPowerConsumptionIdle)) ; If we have Estimated round trip
      (bind _output_get_2 (Variables|Default|SetTripTime (Class|FGDroneStationInfo|GetEstimatedRoundTripTime (Class|FGBuildableDroneStation|GetInfo self))))
      (CallFunction|DEBUG (Utilities|String|Append "Trip Time (estimated): " (Utilities|String|ToString(Float) _output_get_2)) true "(R=0.000000,G=0.031200,B=0.375000,A=1.000000)")
      (goto _label)
      (else
        (CallFunction|DEBUG "No Trip time available yet, wait for next trip to the home port..." true "(R=0.000000,G=0.031200,B=0.375000,A=1.000000)")))))

(fn ConstructionScript
  (|CallParentFunction))